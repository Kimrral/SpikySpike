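; BP_SSCameraComponent is a camera component that keeps framing its owning character and a ball actor together.
; On BeginPlay it resolves the ball by "Ball" tag, records their starting distance, then detaches to move in world space.
; Each Tick it sits along world X from their midpoint, looking at it.
; The offset scales the base arm length by current versus starting distance, clamped between minimum and maximum lengths.
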(event EventBeginPlay
  (CallFunction|Initialize)
  (Transformation|DetachFromComponent "KeepWorld" "KeepWorld" "KeepRelative" true))

(event EventTick
  (params (DeltaSeconds :type Float%20%28single-precision%29))
  (bind _center (CallFunction|GetCenterPoint))
  ;[1 1 1] Update camera location to (center point + dynamic arm length)
  (Transformation|SetWorldLocation (+ _center (Math|Vector|MakeVector (CallFunction|GetCurrentArmLength) 0.0 0.0)) false false)
  ;[1 1 1] Camera to look center point
  (Transformation|SetWorldRotation (Math|Rotator|FindLookatRotation (Transformation|GetWorldLocation) _center) false false))

(fn Initialize
  (params (In%20Ball%20Actor :type Actor%20Object%20Reference))
  (Utilities|IsValid In%20Ball%20Actor
    (:Is%20Valid
      (Variables|Default|SetBall%20Actor In%20Ball%20Actor))
    (:Is%20Not%20Valid
      ;[1 1 1] Ball need 'Ball' Tag
      (bind _outactors (Actor|GetAllActorswithTag "Ball"))
      (bind _array_element (Utilities|Array|ForEachLoopwithBreak _outactors :!label _label)
        (:LoopBody
          (Variables|Default|SetBall%20Actor _array_element)
          (goto _label Break))
        (:Completed
          _))))
  (Utilities|IsValid (Variables|Default|GetCharacter%20Actor)
    (:Is%20Valid
      _)
    (:Is%20Not%20Valid
      (bind _output_get (Variables|Default|SetCharacter%20Actor (Components|GetOwner)))))
  (Variables|Default|SetBase%20Distance (Transformation|GetDistanceTo _output_get (Variables|Default|GetBall%20Actor))))

(fn GetCenterPoint
  (bind _character_actor (Variables|Default|GetCharacter%20Actor))
  (bind _ball_actor (Variables|Default|GetBall%20Actor))
  (Utilities|IsValid _character_actor
    (:Is%20Valid
      (Utilities|IsValid _ball_actor
        (:Is%20Valid
          (return (/ (+ (Transformation|GetActorLocation _character_actor) (Transformation|GetActorLocation _ball_actor)) (Math|Float|MakeLiteralFloat 2.0))))
        (:Is%20Not%20Valid
          _)))
    (:Is%20Not%20Valid
      _))
  (Development|PrintString "[BP_SSCameraComponent - Get Center Point] Character or Balll is NOT VALID !!")
  (return "0, 0, 0"))

(fn GetCurrentArmLength
  (return (Math|Float|Clamp(Float) (* (Variables|Default|GetBase%20Arm%20Length) (/ (Transformation|GetDistanceTo (Variables|Default|GetCharacter%20Actor) (Variables|Default|GetBall%20Actor)) (Variables|Default|GetBase%20Distance))) (Variables|Default|GetMin%20Arm%20Length) (Variables|Default|GetMax%20Arm%20Length))))