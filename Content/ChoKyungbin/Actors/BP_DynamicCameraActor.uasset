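; Dynamic camera actor that keeps the player's pawn and the ball framed as the distance between them changes.
; BeginPlay retries Initialize on a short delay until it finds the "Ball"-tagged actor and the controlled pawn, recording their starting distance.
; Each Tick places it on a world-X offset from their midpoint, facing that point.
; The offset scales the base arm length by current-to-starting distance, clamped to limits.
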(event EventBeginPlay
  (CallFunction|Initialize :!label _label)
  (Utilities|IsValid (Variables|Default|GetBall%20Actor)
    (:Is%20Valid
      (Utilities|IsValid (Variables|Default|GetCharacter%20Actor)
        (:Is%20Not%20Valid
          _)))
    (:Is%20Not%20Valid
      _))
  (Utilities|FlowControl|Delay 0.03)
  (goto _label))

(event Collision|EventActorBeginOverlap
  (params (OtherActor :type Actor%20Object%20Reference)))

(event EventTick
  (params (DeltaSeconds :type Float%20%28single-precision%29))
  (bind _center (CallFunction|GetCenterPoint))
  ;[1 1 1] Update camera location to (center point + dynamic arm length)
  (Transformation|SetActorLocation (+ _center (Math|Vector|MakeVector (CallFunction|GetCurrentArmLength) 0.0 0.0)) false false)
  ;[1 1 1] Camera to look center point
  (Transformation|SetActorRotation (Math|Rotator|FindLookatRotation (Transformation|GetActorLocation) _center)))

(fn ConstructionScript)

(fn Initialize
  ;[1 1 1] Ball need 'Ball' Tag
  (bind _outactors (Actor|GetAllActorswithTag "Ball"))
  (bind _array_element (Utilities|Array|ForEachLoopwithBreak _outactors :!label _label)
    (:LoopBody
      (Variables|Default|SetBall%20Actor _array_element)
      (goto _label Break))
    (:Completed
      (Utilities|IsValid (Variables|Default|GetBall%20Actor)
        (:Is%20Valid
          (bind _output_get (Variables|Default|SetCharacter%20Actor (Pawn|GetControlledPawn (Game|GetPlayerController 0))))
          (Utilities|IsValid _output_get
            (:Is%20Valid
              (Variables|Default|SetBase%20Distance (Transformation|GetDistanceTo (Variables|Default|GetCharacter%20Actor) (Variables|Default|GetBall%20Actor))))
            (:Is%20Not%20Valid
              (return))))
        (:Is%20Not%20Valid
          (return))))))

(fn GetCenterPoint
  (bind _character_actor (Variables|Default|GetCharacter%20Actor))
  (bind _ball_actor (Variables|Default|GetBall%20Actor))
  (Utilities|IsValid _character_actor
    (:Is%20Valid
      (Utilities|IsValid _ball_actor
        (:Is%20Valid
          (return (/ (+ (Transformation|GetActorLocation _character_actor) (Transformation|GetActorLocation _ball_actor)) (Math|Float|MakeLiteralFloat 2.0))))
        (:Is%20Not%20Valid
          _)))
    (:Is%20Not%20Valid
      _))
  (Development|PrintString "[BP_SSCameraComponent - Get Center Point] Character or Balll is NOT VALID !!")
  (return "0, 0, 0"))

(fn GetCurrentArmLength
  (bind _ball_actor (Variables|Default|GetBall%20Actor))
  (bind _character_actor (Variables|Default|GetCharacter%20Actor))
  (Utilities|IsValid _character_actor
    (:Is%20Valid
      (Utilities|IsValid _ball_actor
        (:Is%20Valid
          (return (Math|Float|Clamp(Float) (* (Variables|Default|GetBase%20Arm%20Length) (/ (Transformation|GetDistanceTo _character_actor _ball_actor) (Variables|Default|GetBase%20Distance))) (Variables|Default|GetMin%20Arm%20Length) (Variables|Default|GetMax%20Arm%20Length))))
        (:Is%20Not%20Valid
          _)))
    (:Is%20Not%20Valid
      _))
  (return (Variables|Default|GetBase%20Arm%20Length)))