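; BP_Shark is a shark actor that moves its skeletal mesh along its spline in a continuous loop.
; Each Tick advances a distance by SplineSpeed scaled by delta time, wrapping to zero past the spline's end.
; The mesh takes only the spline's local-space location and keeps its own scale, so it does not turn to follow the path.
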(event EventBeginPlay)

(event Collision|EventActorBeginOverlap
  (params (OtherActor :type Actor%20Object%20Reference)))

(event EventTick
  (params (DeltaSeconds :type Float%20%28single-precision%29))
  (Variables|Default|SetDistanceAlongSpline (+ (* DeltaSeconds (Variables|Default|GetSplineSpeed)) (Variables|Default|GetDistanceAlongSpline)))
  (Transformation|SetRelativeTransform (Variables|Default|GetSkeletalMesh) (Math|Transform|MakeTransform (.location (Spline|GetTransformatDistanceAlongSpline (Variables|Default|GetSpline) (Variables|Default|GetDistanceAlongSpline) "Local" false)) "0, 0, 0" (Variables|/Script/Engine.SceneComponent|GetRelativeScale3D (Variables|Default|GetSkeletalMesh))) false false)
  (if (> (Variables|Default|GetDistanceAlongSpline) (Spline|GetSplineLength (Variables|Default|GetSpline)))
    (Variables|Default|SetDistanceAlongSpline 0.0)))

(fn ConstructionScript)